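; Enemy character that roams random reachable points within a radius and chases the player on sight via PawnSensing, unless the player is hiding.
; Sightings play a found cue gated by a resettable DoOnce, and a retriggerable delay returns it to roaming.
; Overlapping an unhidden player disables the enemy's movement, visibility and collision; a separate event restores them after a delay.
; Ending any overlap uncrouches it, while the overhang crouch check is unwired.
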(event `Disable Enemy`
  ;[1 1 1] Disable Enemy
  (`CharacterMovementComponent.SetMovementMode` (`self.CharacterMovement`) "MOVE_None" 0)
  (`self.SetActorHiddenInGame` true)
  (`PrimitiveComponent.SetCollisionEnabled` (`self.CapsuleComponent`) "NoCollision")
  (set `PrimitiveComponent.bGenerateOverlapEvents` false (`self.BoxCollision`)))

(event `self.ReceiveBeginPlay`
  ;[1 1 1] Roaming code
  (`KismetSystemLibrary.Delay` 3.0)
  (`self.Roaming`))

(event `Roaming`
  ;[1 1 1] Roaming code
  (if (not (`self.PlayerDead`))
    (bind _outactors (`GameplayStatics.GetAllActorsOfClass` "/Game/Blueprints/WallOverhang.WallOverhang_C"))
    (`PrimitiveComponent.IgnoreActorWhenMoving` (`self.BoxCollision`) (`|GetArrayItem` _outactors) false)
    (`|AIMoveTo` self (`NavigationSystemV1.K2_GetRandomReachablePointInRadius` (`self.K2_GetActorLocation`) 2500.0 null null) null
      (:`OnSuccess`
        _)
      (:`OnFail`
        _))
    (`self.Roaming`)))

(event `Reenable Enemy`
  ;[1 1 1] Re-enable Enemy
  (`KismetSystemLibrary.Delay` 10.0)
  (`CharacterMovementComponent.SetMovementMode` (`self.CharacterMovement`) "MOVE_Walking" 0)
  (`self.SetActorHiddenInGame` false)
  (set `PrimitiveComponent.bGenerateOverlapEvents` true (`self.BoxCollision`))
  (`PrimitiveComponent.SetCollisionEnabled` (`self.CapsuleComponent`) "QueryAndPhysics"))

(event `self.PawnSensing.OnSeePawn`
  (params (Pawn :type "Pawn Object Reference"))
  ;[1 1 1] Chasing code
  (bind _asbp_player_character (cast `/Game/Player/Blueprints/BP_PlayerCharacter` Pawn))
  (if (`/Game/Player/Blueprints/BP_PlayerCharacter.IsHiding` _asbp_player_character)
    (`self.Roaming`)
    (else
      (`|ExecutionSequence`
        (:`then_0`
          (`|ExecutionSequence`
            (:`then_0`
              (`/Engine/EditorBlueprintResources/StandardMacros.DoOnce` false :!label _label
                (:`Completed`
                  (`GameplayStatics.PlaySoundAtLocation` "/Game/Audio/Cues/Enemy_found_cue.Enemy_found_cue" (`self.K2_GetActorLocation`) (struct) 1.0 1.0 0.0 null null null null))))
            (:`then_1`
              (`KismetSystemLibrary.RetriggerableDelay` 1.0)
              (goto _label :!via `Reset`))))
        (:`then_1`
          (`|ExecutionSequence`
            (:`then_0`
              (`|AIMoveTo` self (0.0 0.0 0.0) Pawn))
            (:`then_1`
              (`KismetSystemLibrary.RetriggerableDelay` 1.0)
              (`self.Roaming`))))))))

(event `self.ReceiveActorBeginOverlap`
  (params (OtherActor :type "Actor Object Reference"))
  ;[1 1 1] When Player is Hiding + When Enemy reaches an obstacle
  (if (`self.ActorHasTag` OtherActor "Player")
    (bind _asbp_player_character (cast `/Game/Player/Blueprints/BP_PlayerCharacter` OtherActor))
    (if (not (`/Game/Player/Blueprints/BP_PlayerCharacter.IsHiding` _asbp_player_character))
      (`self.Disable Enemy`))))

(event `self.ReceiveActorEndOverlap`
  (params (OtherActor :type "Actor Object Reference"))
  (`self.UnCrouch`))

(fn `UserConstructionScript`)