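; InWorld_Text is an in-world help-text actor whose widget component turns to face the player.
; On BeginPlay it caches the BP_PlayerCharacter, makes the widget visible and starts a looping timer instead of using Tick.
; Each timer call sets the widget's yaw from a look-at rotation toward the player's capsule, zeroing pitch and roll.
; Sphere overlap logic for proximity-based show and hide is disconnected and unused.
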(event `self.ReceiveBeginPlay`
  ;[1 1 1] Rotate help-text to face the player
  (`|ExecutionSequence`
    (:`then_0`
      (bind _asbp_player_character (cast `/Game/Player/Blueprints/BP_PlayerCharacter` (`GameplayStatics.GetPlayerCharacter` 0)))
      (set `self.As BP Player Character` _asbp_player_character)
      (`SceneComponent.SetVisibility` (`self.Widget`) true false))
    (:`then_1`
      (`KismetSystemLibrary.K2_SetTimerDelegate` (delegate `Spinning`) 0.1 true))))

(event `Spinning`
  (bind _widget (`self.Widget`))
  (bind (_returnvalue_roll _returnvalue_pitch _returnvalue_yaw) (`KismetMathLibrary.BreakRotator` (`KismetMathLibrary.FindLookAtRotation` (`SceneComponent.K2_GetComponentLocation` _widget) (`SceneComponent.K2_GetComponentLocation` (`Character.CapsuleComponent` (`self.As BP Player Character`))))))
  ;[1 1 1] Rotate help-text to face the player
  (`SceneComponent.K2_SetWorldRotation` _widget (`KismetMathLibrary.MakeRotator` 0.0 0.0 _returnvalue_yaw) false false))

(event `self.SphereCollision.OnComponentBeginOverlap`
  (params (OverlappedComponent :type "PrimitiveComponent Object Reference") (OtherActor :type "Actor Object Reference") (OtherComp :type "PrimitiveComponent Object Reference") (OtherBodyIndex :type Integer) (bFromSweep :type Boolean) (SweepResult :type "HitResult Structure (by ref)"))
  ;[1 1 1] When Player is near the text trigger, display text NOT IN USE
)

(event `self.SphereCollision.OnComponentEndOverlap`
  (params (OverlappedComponent :type "PrimitiveComponent Object Reference") (OtherActor :type "Actor Object Reference") (OtherComp :type "PrimitiveComponent Object Reference") (OtherBodyIndex :type Integer))
  ;[1 1 1] When Player is near the text trigger, display text NOT IN USE
)

(fn `UserConstructionScript`)