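; Temporary guide arrow that turns to point toward the exit censer, then destroys itself after ten seconds.
; BeginPlay sets a neutral rotation and stores the look-at rotation toward the first Checkpoint_Censer_BP found in the level.
; Until its rotation is within tolerance of that target, Tick adds a fixed yaw step and lowers the arrow slightly each frame, independent of delta time.
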(event `self.ReceiveBeginPlay`
  ;[1 1 1] When Arrow constructed, set to neutral rotate position, and find position of exit censer to looks at. After 10 seconds destroy Arrow
  (`self.K2_SetActorRotation` (struct :`Yaw` -90.0))
  (bind _outactors (`GameplayStatics.GetAllActorsOfClass` "/Game/Blueprints/Key_Objects/Censers/Checkpoint_Censer_BP.Checkpoint_Censer_BP_C"))
  (set `self.RotateTo` (`KismetMathLibrary.FindLookAtRotation` (`SceneComponent.K2_GetComponentLocation` (`self.DefaultSceneRoot`)) (`SceneComponent.K2_GetComponentLocation` (`/Game/Blueprints/Key_Objects/Censers/Checkpoint_Censer_BP.Censer Mesh` (`|GetArrayItem` _outactors)))))
  (`KismetSystemLibrary.Delay` 10.0)
  (`self.K2_DestroyActor`))

(event `self.ReceiveTick`
  (params (DeltaSeconds :type "Float (single-precision)"))
  (bind _defaultsceneroot (`self.DefaultSceneRoot`))
  ;[1 1 1] Animate the Arrow to rotate to look at where the exit censer is
  (if (!= (`SceneComponent.K2_GetComponentRotation` (`self.DefaultSceneRoot`)) (`self.RotateTo`) :`ErrorTolerance` 10.0)
    (`SceneComponent.K2_AddRelativeRotation` _defaultsceneroot (`KismetMathLibrary.MakeRotator` 0.0 0.0 2.0) false false)
    (`SceneComponent.K2_AddRelativeLocation` _defaultsceneroot (0.0 0.0 -1.0) false false)))

(fn `UserConstructionScript`)